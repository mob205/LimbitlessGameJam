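; Rune password puzzle actor that generates a three-stage orientation code and checks rotations submitted by up to four players.
; BeginPlay rolls three unique cube faces and three rune spins, which SetRotation applies to the target and rune components.
; RetrieveRotationFromCube advances that player's marker visuals, comparing normalized rotation to the stage target within 40 degrees only once the player's marker flag is set.
; Debug prints and disconnected randomization logic remain.
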(event `WhatSide`
  (bind _returnvalue (`KismetArrayLibrary.Array_AddUnique` (`self.Side`) (`KismetMathLibrary.RandomIntegerInRange` 0 5)))
  (if (== _returnvalue -1)
    (`self.WhatSide`)))

(event `WhatRotation`
  (`KismetArrayLibrary.Array_Add` (`self.Rotation`) (`KismetMathLibrary.RandomIntegerInRange` 0 3)))

(event `self.ReceiveBeginPlay`
  (`self.WhatSide`)
  (`self.WhatSide`)
  (`self.WhatSide`)
  (`self.WhatRotation`)
  (`self.WhatRotation`)
  (`self.WhatRotation`)
  (`self.SetRotation` 0)
  (`self.SetRotation` 1)
  (`self.SetRotation` 2)
  (`|ExecutionSequence`
    (:`then_0`
      (for _array_element (`|MakeArray` (`self.P1M1`) (`self.P4M1`) (`self.P2M1`) (`self.P3M1`) (`self.P1M2`) (`self.P4M2`) (`self.P3M2`) (`self.P2M2`))
        (`SceneComponent.SetVisibility` _array_element false false))
      (`KismetSystemLibrary.PrintString` "KILL YOURSELF"))))

(fn `Retrieve Rotation from Cube`
  (params (`Submitted Rotation` :type "Rotator Structure") (WhichStage :type Integer) (WhichPlayer :type Integer))
  (returns (Result :type Boolean))
  (bind _returnvalue (`KismetMathLibrary.MakeRotator` (`KismetMathLibrary.NormalizeAxis` (.roll `Submitted Rotation`)) (`KismetMathLibrary.NormalizeAxis` (.pitch `Submitted Rotation`)) (`KismetMathLibrary.NormalizeAxis` (.yaw `Submitted Rotation`))))
  (bind _returnvalue_2 (`KismetMathLibrary.MakeRotator` (`KismetMathLibrary.NormalizeAxis` (.roll (`SceneComponent.K2_GetComponentRotation` (`|GetArrayItem` (`|MakeArray` (`self.PasswordTarget1`) (`self.PasswordTarget2`) (`self.PasswordTarget3`)) WhichStage)))) (`KismetMathLibrary.NormalizeAxis` (.pitch (`SceneComponent.K2_GetComponentRotation` (`|GetArrayItem` (`|MakeArray` (`self.PasswordTarget1`) (`self.PasswordTarget2`) (`self.PasswordTarget3`)) WhichStage)))) (`KismetMathLibrary.NormalizeAxis` (.yaw (`SceneComponent.K2_GetComponentRotation` (`|GetArrayItem` (`|MakeArray` (`self.PasswordTarget1`) (`self.PasswordTarget2`) (`self.PasswordTarget3`)) WhichStage))))))
  (bind _returnvalue_3 (== _returnvalue _returnvalue_2 :`ErrorTolerance` 40.0))
  (`|ExecutionSequence`
    (:`then_0`
      (switch `int` WhichPlayer
        (:`0`
          (if (`self.P1Marker`)
            (`SceneComponent.SetVisibility` (`self.P1M1`) false false)
            (`SceneComponent.SetVisibility` (`self.P1M2`) true false)
            (return _returnvalue_3)
            (else
              (set `self.P1Marker` true)
              (`SceneComponent.SetVisibility` (`self.P1M3`) false false)
              (`SceneComponent.SetVisibility` (`self.P1M1`) true false))))
        (:`1`
          (if (`self.P2Marker`)
            (`SceneComponent.SetVisibility` (`self.P2M1`) false false)
            (`SceneComponent.SetVisibility` (`self.P2M2`) true false)
            (return _returnvalue_3)
            (else
              (set `self.P2Marker` true)
              (`SceneComponent.SetVisibility` (`self.P2M3`) false false)
              (`SceneComponent.SetVisibility` (`self.P2M1`) true false))))
        (:`2`
          (if (`self.P3Marker`)
            (`SceneComponent.SetVisibility` (`self.P3M1`) false false)
            (`SceneComponent.SetVisibility` (`self.P3M2`) true false)
            (return _returnvalue_3)
            (else
              (set `self.P3Marker` true)
              (`SceneComponent.SetVisibility` (`self.P3M3`) false false)
              (`SceneComponent.SetVisibility` (`self.P3M1`) true false))))
        (:`3`
          (if (`self.P4Marker`)
            (`SceneComponent.SetVisibility` (`self.P4M1`) false false)
            (`SceneComponent.SetVisibility` (`self.P4M2`) true false)
            (return _returnvalue_3)
            (else
              (set `self.P4Marker` true)
              (`SceneComponent.SetVisibility` (`self.P4M3`) false false)
              (`SceneComponent.SetVisibility` (`self.P4M1`) true false))))))
    (:`then_1`
      (`KismetSystemLibrary.PrintString` (`KismetStringLibrary.Conv_RotatorToString` _returnvalue_2) true true (struct :`R` 1.0 :`B` 0.231755 :`A` 1.0))
      (`KismetSystemLibrary.PrintString` (`KismetStringLibrary.Conv_RotatorToString` _returnvalue) true true (struct :`G` 1.0 :`B` 0.003757 :`A` 1.0))
      (`KismetSystemLibrary.PrintString` (`KismetStringLibrary.Conv_IntToString` WhichStage) true true (struct :`R` 0.221679 :`B` 1.0 :`A` 1.0))
      (if _returnvalue_3
        _))))

(fn `SetRotation`
  (params (Cube :type Integer))
  (`SceneComponent.K2_SetRelativeRotation` (`|GetArrayItem` (`|MakeArray` (`self.PasswordTarget1`) (`self.PasswordTarget2`) (`self.PasswordTarget3`)) Cube) (select `int` (`|GetArrayItem` (`self.Side`) Cube) :`0` (struct) :`1` (struct :`Yaw` 90.0) :`2` (struct :`Yaw` 180.0) :`3` (struct :`Yaw` -90.0) :`4` (struct :`Pitch` 90.0) :`5` (struct :`Pitch` -90.0) :!type "Rotator Structure") false false)
  (`SceneComponent.K2_SetRelativeRotation` (`|GetArrayItem` (`|MakeArray` (`self.Rune1`) (`self.Rune2`) (`self.Rune3`)) Cube) (`KismetMathLibrary.MakeRotator` (select `int` (`|GetArrayItem` (`self.Rotation`) Cube) :`0` 0.0 :`1` -90.0 :`2` -180.0 :`3` 90.0 :!type "Float (single-precision)")) false false))

(fn `UserConstructionScript`)