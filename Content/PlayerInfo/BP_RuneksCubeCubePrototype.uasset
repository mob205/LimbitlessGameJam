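; BP_RuneksCubeCubePrototype is a prototype rotating-cube input for a rune password puzzle, tracked per player number.
; Held spin inputs run repeat timelines that trigger eased right or down rotation steps, gated by AnimationIsPlaying; only the right spin snaps to its target on finish.
; Button 3 submits the cube's rotation and stage index to BP_RunePassword; a match increments the stage and calls Schmoove, with debug prints for either result.
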(event `InputAction|SpinRight`
  (params (Key :type "Key Structure"))
  (:`Pressed`
    (`Timeline|RepeatTimer` :!via `PlayFromStart` :!label _label
      (:`Update`
        (`self.RepeatActionSpinRight`))))
  (:`Released`
    (goto _label :!via `Stop`)))

(event `InputAction|spinDown`
  (params (Key :type "Key Structure"))
  (:`Pressed`
    (`Timeline|Timeline_1` :!via `PlayFromStart` :!label _label_2
      (:`Update`
        (`self.RepeatActionSpinDown`))))
  (:`Released`
    (goto _label_2 :!via `Stop`)))

(event `RepeatActionSpinDown`
  (bind _relative_rotation (`self.Relative Rotation`))
  (if (not (`self.AnimationIsPlaying`))
    (set `self.Relative Rotation` (`SceneComponent.RelativeRotation` (`self.Cube`)))
    (bind (_direction _newtrack_0) (`Timeline|Timeline` :!via `PlayFromStart`)
      (:`Update`
        (set `self.AnimationIsPlaying` true)
        (`SceneComponent.K2_SetRelativeRotation` (`self.Cube`) (`KismetMathLibrary.RLerp` _relative_rotation (`KismetMathLibrary.ComposeRotators` _relative_rotation (`KismetMathLibrary.MakeRotFromY` (`self.RotFromY`))) _newtrack_0 true) false false))
      (:`Finished`
        (`|ExecutionSequence`
          (:`then_0`
            (set `self.AnimationIsPlaying` false)))))))

(event `RepeatActionSpinRight`
  (bind _cube (`self.Cube`))
  (bind _relative_rotation (`self.Relative Rotation`))
  (bind _returnvalue (`KismetMathLibrary.ComposeRotators` _relative_rotation (`KismetMathLibrary.MakeRotFromZ` (`self.RotFromZ`))))
  (if (not (`self.AnimationIsPlaying`))
    (set `self.Relative Rotation` (`SceneComponent.RelativeRotation` (`self.Cube`)))
    (bind (_direction _newtrack_0) (`Timeline|Timeline_0` :!via `PlayFromStart`)
      (:`Update`
        (set `self.AnimationIsPlaying` true)
        (`SceneComponent.K2_SetRelativeRotation` _cube (`KismetMathLibrary.RLerp` _relative_rotation _returnvalue _newtrack_0 true) false false))
      (:`Finished`
        (`|ExecutionSequence`
          (:`then_0`
            (set `self.AnimationIsPlaying` false))
          (:`then_1`
            (`SceneComponent.K2_SetRelativeRotation` _cube _returnvalue false false)))))))

(event `EnhancedInput|/MinigameCore/Input/IA_Button3`
  (params (ActionValue :type Boolean) (ElapsedSeconds :type "Float (double-precision)") (TriggeredSeconds :type "Float (double-precision)") (InputAction :type "InputAction Object Reference" :default "/MinigameCore/Input/IA_Button3.IA_Button3"))
  (bind _indexer (`self.Indexer`))
  (:`Started`
    (if (not (`self.AnimationIsPlaying`))
      (bind _returnvalue (`GameplayStatics.GetActorOfClass` "/Game/PlayerInfo/BP_RunePassword.BP_RunePassword_C"))
      (bind _result (`/Game/PlayerInfo/BP_RunePassword.Retrieve Rotation from Cube` _returnvalue (`SceneComponent.RelativeRotation` (`self.Cube`)) _indexer (`self.PlayerNumber`)))
      (if _result
        (bind _result_2 (`/Engine/EditorBlueprintResources/StandardMacros.IncrementInt` _indexer)
          (:`  `
            (`KismetSystemLibrary.PrintString` (`KismetStringLibrary.Conv_IntToString` _result_2))
            (`KismetSystemLibrary.PrintString` "RÄT")
            (bind _returnvalue_2 (`GameplayStatics.GetActorOfClass` "/Game/PlayerInfo/BP_RunePassword.BP_RunePassword_C"))
            (`/Game/PlayerInfo/BP_RunePassword.Schmoove` _returnvalue_2 (`self.PlayerNumber`))))
        (else
          (`KismetSystemLibrary.PrintString` "FÄLL"))))))

(fn `UserConstructionScript`)